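; Side-scrolling flipbook player character that runs, jumps and can invert gravity, using Enhanced Input.
; Movement input follows the actor's forward vector, switching run and idle flipbooks and rotating the sprite to face the travel direction.
; Jumping sets a flag and polls vertical velocity on a short delay loop to detect landing.
; Gravity swap only toggles a flag, which Tick reads to set gravity direction and sprite rotation every frame.
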(event Input|EnhancedActionEvents|EnhancedInputActionIA_Move
  (params (ActionValue :type Float%20%28double-precision%29) (ElapsedSeconds :type Float%20%28double-precision%29) (TriggeredSeconds :type Float%20%28double-precision%29) (InputAction :type Input%20Action%20Object%20Reference :default "/Game/Blueprints/IA_Move.IA_Move"))
  (bind _sprite (Variables|Default|GetSprite))
  (:Triggered
    (Pawn|Input|AddMovementInput (Transformation|GetActorForwardVector) ActionValue false)
    (if (Variables|Default|GetbIs_Jumping)
      _
      (else
        (Sprite|SetFlipbook (Variables|Default|GetSprite) "/Game/Assets/FB_run.FB_run")))
    (if (> ActionValue 0.0)
      (Transformation|SetWorldRotation _sprite "0, 0, 0" false false)
      (else
        (Transformation|SetWorldRotation _sprite "0.000000,-180.000000,0.000000" false false))))
  (:Completed
    (if (not (Variables|Default|GetbIs_Jumping))
      (Sprite|SetFlipbook (Variables|Default|GetSprite) "/Game/Assets/FB_idle.FB_idle"))))

(event Input|EnhancedActionEvents|EnhancedInputActionIA_Jump
  (params (ActionValue :type Boolean) (ElapsedSeconds :type Float%20%28double-precision%29) (TriggeredSeconds :type Float%20%28double-precision%29) (InputAction :type Input%20Action%20Object%20Reference :default "/Game/Blueprints/IA_Jump.IA_Jump"))
  (bind _sprite (Variables|Default|GetSprite))
  (if (not (Variables|Default|GetbIs_Jumping))
    (Variables|Default|SetbIs_Jumping true)
    (Character|Jump)
    (Components|Timeline|SetLooping _sprite false)
    (Sprite|SetFlipbook _sprite "/Game/Assets/FB_jump.FB_jump")
    (Utilities|FlowControl|Delay 0.1)
    (if (== (.Z (Math|Vector|BreakVector (Transformation|GetVelocity))) 0.0) :!label _label
      (Components|Timeline|SetLooping _sprite false)
      (Audio|Components|Audio|Play _sprite)
      (Sprite|SetFlipbook _sprite "/Game/Assets/FB_idle.FB_idle")
      (Variables|Default|SetbIs_Jumping false)
      (else
        (Utilities|FlowControl|Delay 0.1)
        (goto _label)))))

(event Input|EnhancedActionEvents|EnhancedInputActionIA_Gravity_Swap
  (params (ActionValue :type Boolean) (ElapsedSeconds :type Float%20%28double-precision%29) (TriggeredSeconds :type Float%20%28double-precision%29) (InputAction :type Input%20Action%20Object%20Reference :default "/Game/Blueprints/IA_Gravity_Swap.IA_Gravity_Swap"))
  (bind _output_get (Variables|Default|SetbToggle_Gravity (not (Variables|Default|GetbToggle_Gravity))))
  (if _output_get
    _))

(event EventBeginPlay
  (bind _asbp_player_controller (Utilities|Casting|CastToBP_PlayerController (Pawn|GetController)))
  (Input|AddMappingContext (PlayerController|LocalPlayerSubsystems|GetEnhancedInputLocalPlayerSubsystem _asbp_player_controller) "/Game/Blueprints/IMC_Default.IMC_Default" 0 "(bIgnoreAllPressedKeysUntilRelease=True,bForceImmediately=False,bNotifyUserSettings=False)"))

(event EventTick
  (params (DeltaSeconds :type Float%20%28single-precision%29))
  (bind _sprite (Variables|Default|GetSprite))
  (bind _returnvalue (Transformation|GetWorldRotation _sprite))
  (if (Variables|Default|GetbToggle_Gravity)
    (Class|CharacterMovementComponent|SetGravityDirection (Variables|Character|GetCharacterMovement) (Math|Vector|MakeVector 0.0 0.0 1.0))
    (Transformation|SetWorldRotation _sprite (Math|Rotator|MakeRotator 0.0 1.8e+02 (+ (.yaw _returnvalue) 1.8e+02)) false false)
    (else
      (Class|CharacterMovementComponent|SetGravityDirection (Variables|Character|GetCharacterMovement) (Math|Vector|MakeVector 0.0 0.0 -1.0))
      (Transformation|SetWorldRotation _sprite (Math|Rotator|MakeRotator 0.0 0.0 (.yaw _returnvalue)) false false))))

(fn ConstructionScript)